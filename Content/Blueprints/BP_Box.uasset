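; BP_Box is a box actor that yaws its mesh 90 degrees on each Enter press and updates which side materials are tinted.
; BeginPlay enables input and stores dynamic instances of material slots 1 to 4.
; SetValueWithLoop wraps the current and next side indices.
; Those two materials get a zero V1_BaseColorTint and the others one, which comments describe as setting front and right opacity.
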(event `self.ReceiveBeginPlay`
  (bind _sm_box (`self.SM_Box`))
  ;[1 1 1] Enabling Input
  (`self.EnableInput` (`GameplayStatics.GetPlayerController` 0))
  ;[1 1 1] Constructing Dynamic Material Instances
  (for _index (range 1 5)
    (bind _returnvalue (`PrimitiveComponent.CreateDynamicMaterialInstance` _sm_box _index (`PrimitiveComponent.GetMaterial` _sm_box _index) "None"))
    (`KismetArrayLibrary.Array_Add` (`self.Materials`) _returnvalue)))

(event `Key|Enter`
  (params (Key :type "Key Structure"))
  (bind _sm_box (`self.SM_Box`))
  (bind (_relativerotation_roll _relativerotation_pitch _relativerotation_yaw) (`KismetMathLibrary.BreakRotator` (`SceneComponent.RelativeRotation` _sm_box)))
  (:`Pressed`
    ;[1 1 1] Rotate Box
    (`SceneComponent.K2_SetRelativeRotation` _sm_box (`KismetMathLibrary.MakeRotator` _relativerotation_roll _relativerotation_pitch (+ _relativerotation_yaw 90.0)) false false)
    ;[1 1 1] Incrementing Rotation Index
    (bind _output (`self.SetValueWithLoop` (`self.CurrentRotationIndex`) 1 0 3))
    (bind _output_get (set `self.CurrentRotationIndex` _output))
    (bind _output_2 (`self.SetValueWithLoop` _output_get 1 0 3))
    (set `self.NexRotationIndex` _output_2)
    ;[1 1 1] Setting Opacity By Front And Right Materials
    (for (_array_element _array_index) (`self.Materials`)
      (if (or (== _array_index (`self.CurrentRotationIndex`)) (== _array_index (`self.NexRotationIndex`)))
        (`MaterialInstanceDynamic.SetScalarParameterValue` _array_element "V1_BaseColorTint" 0.0)
        (else
          (`MaterialInstanceDynamic.SetScalarParameterValue` _array_element "V1_BaseColorTint" 1.0))))))

(fn `SetValueWithLoop`
  (params (Input :type "Integer (by ref)") (Incriment :type Integer :default 1) (StartValue :type Integer) (EndValue :type Integer))
  (returns (Output :type Integer))
  (locals (F_Input :type Integer) (NewLocalVar :type Integer) (F_StartValue :type Integer) (F_EndValue :type Integer))
  ;[1 1 1] Setting Vars
  (set `local.F_Input` (+ Input Incriment))
  (set `local.F_StartValue` StartValue)
  (set `local.F_EndValue` EndValue)
  ;[1 1 1] Checking If Incrimented Input Is bigger than end value
  (if (> (`local.F_Input`) (`local.F_EndValue`))
    ;[1 1 1] Reset Input to start value
    (bind _output_get (set `local.F_Input` (`local.F_StartValue`)))
    (return _output_get)
    (else
      ;[1 1 1] Checking if Incrimented input is less than start value
      (if (< (`local.F_Input`) (`local.F_StartValue`))
        ;[1 1 1] Reset Input to End Value
        (bind _output_get_2 (set `local.F_Input` (`local.F_EndValue`)))
        (return _output_get_2)
        (else
          ;[1 1 1] Return Incrimented Input
          (return (`local.F_Input`)))))))

(fn `UserConstructionScript`)